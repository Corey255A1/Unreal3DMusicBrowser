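; Actor that builds an in-world music browser from Emby genres, artists, albums and songs, each shown as a spawned BP_MusicPillar with name and image.
; Add functions space pillars along per-level offsets, tag them by level and store song URLs as extra data.
; SelectPillar reads the tag, moves the fire highlight to the chosen pillar, destroys lower-level pillars and calls that level's Selected event with the name, plus URL for songs.
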(event EventBeginPlay)

(fn ConstructionScript)

(fn AddGenre
  (params (EmbyObject :type Emby%20Object%20Structure))
  (bind (_name _primaryimageurl) (Utilities|Struct|BreakEmbyObject EmbyObject))
  (bind _new_pilar (CallFunction|AddPillar (Utilities|Text|ToText(String) _name) "" (Variables|Default|GetGenreOffset) (Variables|Default|GetGenreObjects) _primaryimageurl))
  (Variables|/Script/Engine.Actor|SetTags _new_pilar (Utilities|Array|MakeArray "Genre")))

(fn AddArtist
  (params (EmbyObject :type Emby%20Object%20Structure))
  (bind (_name _primaryimageurl) (Utilities|Struct|BreakEmbyObject EmbyObject))
  (bind _new_pilar (CallFunction|AddPillar (Utilities|Text|ToText(String) _name) "" (Variables|Default|GetArtistOffset) (Variables|Default|GetArtistObjects) _primaryimageurl))
  (Variables|/Script/Engine.Actor|SetTags _new_pilar (Utilities|Array|MakeArray "Artist")))

(fn AddAlbum
  (params (EmbyObject :type Emby%20Object%20Structure))
  (bind (_name _primaryimageurl) (Utilities|Struct|BreakEmbyObject EmbyObject))
  (bind _new_pilar (CallFunction|AddPillar (Utilities|Text|ToText(String) _name) "" (Variables|Default|GetAlbumOffset) (Variables|Default|GetAlbumObjects) _primaryimageurl))
  (Variables|/Script/Engine.Actor|SetTags _new_pilar (Utilities|Array|MakeArray "Album")))

(fn AddSong
  (params (EmbySong :type Emby%20Song%20Structure))
  (bind (_url _name _primaryimageurl) (Utilities|Struct|BreakEmbySong EmbySong))
  (bind _new_pilar (CallFunction|AddPillar (Utilities|Text|ToText(String) _name) _url (Variables|Default|GetSongOffset) (Variables|Default|GetSongObjects) _primaryimageurl))
  (Variables|/Script/Engine.Actor|SetTags _new_pilar (Utilities|Array|MakeArray "Song")))

(fn AddPillar
  (params (Label :type Text) (ExtraData :type String) (Offset :type Transform) (PillarArray :type Array%20of%20BP%20Music%20Pillar%20Object%20References) (ImageURL :type String))
  (bind _returnvalue (Transformation|GetActorTransform))
  (bind _returnvalue_2 (Game|SpawnActorfromClass "/Game/BP_MusicPillar.BP_MusicPillar_C" (Math|Transform|MakeTransform (+ (+ (.location Offset) (* (Variables|Default|GetPilarSpacingOffset) (Utilities|Array|Length PillarArray))) (.location _returnvalue)) (.rotation _returnvalue) (.scale _returnvalue)) "Undefined" "MultiplyWithRoot" 0 0))
  (Variables|/Game/BP_MusicPillar.BP_MusicPillar_C|SetExtraData _returnvalue_2 ExtraData)
  (Default|SetPillarImageURL _returnvalue_2 ImageURL)
  (Default|SetPillarText _returnvalue_2 (Utilities|String|ToString(Text) Label))
  (Utilities|Array|Add PillarArray _returnvalue_2)
  (return _returnvalue_2))

(fn SelectPillar
  (params (Hit%20Pilar :type BP%20Music%20Pillar%20Object%20Reference))
  (LocalVariables|SetHitPilar Hit%20Pilar)
  (if (Actor|ActorHasTag (LocalVariables|GetHitPilar) "Genre")
    (bind _selectedpillar (CallFunction|SwapSelectedPillar Hit%20Pilar (Variables|Default|GetCurrentGenre)))
    (Variables|Default|SetCurrentGenre _selectedpillar)
    (CallFunction|ClearPillarArray (Variables|Default|GetArtistObjects))
    (CallFunction|ClearPillarArray (Variables|Default|GetAlbumObjects))
    (CallFunction|ClearPillarArray (Variables|Default|GetSongObjects))
    (Default|CallGenreSelected (Default|GetPillarText (Variables|Default|GetCurrentGenre)))
    (elif (Actor|ActorHasTag (LocalVariables|GetHitPilar) "Artist")
      (bind _selectedpillar_2 (CallFunction|SwapSelectedPillar Hit%20Pilar (Variables|Default|GetCurrentArtist)))
      (Variables|Default|SetCurrentArtist _selectedpillar_2)
      (CallFunction|ClearPillarArray (Variables|Default|GetAlbumObjects))
      (CallFunction|ClearPillarArray (Variables|Default|GetSongObjects))
      (Default|CallArtistSelected (Default|GetPillarText (Variables|Default|GetCurrentArtist)))
      (elif (Actor|ActorHasTag (LocalVariables|GetHitPilar) "Album")
        (bind _selectedpillar_3 (CallFunction|SwapSelectedPillar Hit%20Pilar (Variables|Default|GetCurrentAlbum)))
        (Variables|Default|SetCurrentAlbum _selectedpillar_3)
        (CallFunction|ClearPillarArray (Variables|Default|GetSongObjects))
        (Default|CallAlbumSelected (Default|GetPillarText (Variables|Default|GetCurrentAlbum)))
        (elif (Actor|ActorHasTag (LocalVariables|GetHitPilar) "Song")
          (bind _selectedpillar_4 (CallFunction|SwapSelectedPillar Hit%20Pilar (Variables|Default|GetCurrentSong)))
          (Variables|Default|SetCurrentSong _selectedpillar_4)
          (Default|CallSongSelected (Default|GetPillarText (Variables|Default|GetCurrentSong)) (Variables|/Game/BP_MusicPillar.BP_MusicPillar_C|GetExtraData (Variables|Default|GetCurrentSong))))))))

(fn SwapSelectedPillar
  (params (HitPilar :type BP%20Music%20Pillar%20Object%20Reference) (CurrentPillar :type BP%20Music%20Pillar%20Object%20Reference))
  (if (Utilities|IsValid CurrentPillar)
    (if (!= HitPilar CurrentPillar)
      (Default|SetFireActive CurrentPillar false)
      (else
        (return CurrentPillar))))
  (Default|SetFireActive HitPilar true)
  (return HitPilar))

(fn ClearPillarArray
  (params (Pillars :type Array%20of%20BP%20Music%20Pillar%20Object%20References))
  (for _array_element Pillars
    (Actor|DestroyActor _array_element))
  (Utilities|Array|Clear Pillars))