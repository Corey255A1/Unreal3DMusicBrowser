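; Game mode that connects an in-level music browser to asynchronous music library queries and media playback.
; On BeginPlay it binds to the genre, artist, album and song selection events of the first BP_MusicBrowserCreator.
; Selections request the next level of artists, albums or songs, and received lists are added to the browser.
; A selected song's URL opens in the first MediaPlate's player and plays once loaded.
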(event Custom|OnGenreSelected
  (params (GenreName :type Text))
  (Class|MusicGameBase|GetArtistsOfGenreAsync (Utilities|String|ToString(Text) GenreName)))

(event Custom|OnAlbumSelected
  (params (AlbumName :type Text))
  (Class|MusicGameBase|GetSongsOfAlbumsAsync (Utilities|String|ToString(Text) (Default|GetPillarText (Variables|/Game/BP_MusicBrowserCreator.BP_MusicBrowserCreator_C|GetCurrentArtist (Variables|Default|GetMusicBrowser)))) (Utilities|String|ToString(Text) AlbumName)))

(event Custom|OnArtistSelected
  (params (ArtistName :type Text))
  (Class|MusicGameBase|GetAlbumsOfArtistsAsync (Utilities|String|ToString(Text) ArtistName)))

(event Custom|OnSongSelected
  (params (SongName :type Text) (URL :type String))
  (Class|MediaPlayer|OpenUrl (Variables|Default|GetMediaPlayer) URL))

(event Custom|OnMediaURLLoaded
  (params (OpenedUrl :type String))
  (Media|MediaPlayer|Play (stale EventBeginPlay _output_get_2) :!class /Script/MediaAssets.MediaPlayer))

(event EventBeginPlay
  (bind _outactors (Actor|GetAllActorsOfClass "/Game/BP_MusicBrowserCreator.BP_MusicBrowserCreator_C"))
  (bind _output_get (Variables|Default|SetMusicBrowser (Utilities|Array|Get(acopy) _outactors)))
  (EventDispatchers|BindEventtoGenreSelected _output_get (delegate Custom|OnGenreSelected))
  (EventDispatchers|BindEventtoAlbumSelected _output_get (delegate Custom|OnAlbumSelected))
  (EventDispatchers|BindEventtoArtistSelected _output_get (delegate Custom|OnArtistSelected))
  (EventDispatchers|BindEventtoSongSelected _output_get (delegate Custom|OnSongSelected))
  (bind _outactors_2 (Actor|GetAllActorsOfClass "/Script/MediaPlate.MediaPlate"))
  (bind _returnvalue (Class|MediaPlateComponent|GetMediaPlayer (Variables|/Script/MediaPlate.MediaPlate|GetMediaPlateComponent (Utilities|Array|Get(acopy) _outactors_2))))
  (bind _output_get_2 (Variables|Default|SetMediaPlayer _returnvalue))
  (Media|MediaPlayer|BindEventtoOnMediaOpened _output_get_2 (delegate Custom|OnMediaURLLoaded)))

(event EventArtistsReceived
  (params (ArtistList :type Array%20of%20Emby%20Object%20Structures))
  (bind _musicbrowser (Variables|Default|GetMusicBrowser))
  ;[1 1 1] Add Artist
  (if (Utilities|IsValid _musicbrowser)
    (for _array_element ArtistList
      (Default|AddArtist _musicbrowser _array_element))))

(event EventGenresReceived
  (params (GenreList :type Array%20of%20Emby%20Object%20Structures))
  (bind _musicbrowser (Variables|Default|GetMusicBrowser))
  ;[1 1 1] Add Genre
  (if (Utilities|IsValid _musicbrowser)
    (for _array_element GenreList
      (Default|AddGenre _musicbrowser _array_element))))

(event EventAlbumsReceived
  (params (AlbumList :type Array%20of%20Emby%20Object%20Structures))
  (bind _musicbrowser (Variables|Default|GetMusicBrowser))
  ;[1 1 1] Add Album
  (if (Utilities|IsValid _musicbrowser)
    (for _array_element AlbumList
      (Default|AddAlbum _musicbrowser _array_element))))

(event EventSongsReceived
  (params (SongList :type Array%20of%20Emby%20Song%20Structures))
  (bind _musicbrowser (Variables|Default|GetMusicBrowser))
  ;[1 1 1] Add Song
  (if (Utilities|IsValid _musicbrowser)
    (for _array_element SongList
      (Default|AddSong _musicbrowser _array_element))))

(fn ConstructionScript)