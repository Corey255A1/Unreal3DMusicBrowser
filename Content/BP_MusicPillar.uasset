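; BP_MusicPillar is a pillar actor that shows a text label and a URL-sourced image, with a fire effect that can be toggled.
; Setting the image URL fires a dispatcher whose handler downloads the image into the Texture parameter of a dynamic material created in the construction script.
; Setting the text stores the raw string and wraps it into short lines joined by break tags for the label.
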(event Custom|EventImageURLChanged
  (params (URL :type String))
  (bind _texture (|DownloadImage URL)
    (:OnSuccess
      (Rendering|Material|SetTextureParameterValue (Variables|Default|GetImageMaterial) "Texture" _texture))))

(event EventBeginPlay
  (EventDispatchers|BindEventtoImageURLChanged (delegate Custom|EventImageURLChanged)))

(fn ConstructionScript
  (bind _returnvalue (Rendering|Material|CreateDynamicMaterialInstance (Variables|Default|GetImage) 0 "/Game/MM_URLImage.MM_URLImage" "None" :!class /Script/Engine.PrimitiveComponent))
  (Variables|Default|SetImageMaterial _returnvalue))

(fn SetFireActive
  (params (FireActive :type Boolean))
  (bind _fire (Variables|Default|GetFire))
  (bind _output_get (Variables|Default|SetIsFireActive FireActive))
  (if _output_get
    (Components|Activation|Activate _fire false)
    (else
      (Components|Activation|Deactivate _fire))))

(fn GetPillarText
  (return (Utilities|Text|ToText(String) (Variables|Default|GetRawText))))

(fn SetPillarText
  (params (Text :type String))
  (bind _output_get (Variables|Default|SetRawText Text))
  (bind _multiline (CallFunction|SplitLineIntoLength 10 _output_get "<br>"))
  (Rendering|Components|TextRender|SetText (Variables|Default|GetLabel) (Utilities|Text|ToText(String) _multiline))
  (return _multiline))

(fn SplitLineIntoLength
  (params (LineLength :type Integer) (Line :type String) (LineDelim :type String))
  (LocalVariables|SetMaxLineLength LineLength)
  (LocalVariables|SetLineJoinDelim LineDelim)
  (for _array_element (Utilities|String|ParseIntoArray Line " ")
    (if (>= (Utilities|String|Len (Utilities|String|Append (LocalVariables|GetCurrentLine) _array_element)) (LocalVariables|GetMaxLineLength))
      (if (Utilities|Array|IsEmpty (LocalVariables|GetCurrentLine))
        _
        (else
          (Utilities|Array|Add (LocalVariables|GetNewString) (LocalVariables|GetCurrentLine))))
      (LocalVariables|SetCurrentLine (Utilities|String|Append _array_element " "))
      (else
        (LocalVariables|SetCurrentLine (Utilities|String|Append (Utilities|String|Append (LocalVariables|GetCurrentLine) _array_element) " ")))))
  (if (not (Utilities|Array|IsEmpty (LocalVariables|GetCurrentLine)))
    (Utilities|Array|Add (LocalVariables|GetNewString) (LocalVariables|GetCurrentLine))
    (return (Utilities|String|JoinStringArray (LocalVariables|GetNewString) (LocalVariables|GetLineJoinDelim)))))

(fn SetPillarImageURL
  (params (URL :type String))
  (bind _output_get (Variables|Default|SetImageURL URL))
  (Default|CallImageURLChanged _output_get))